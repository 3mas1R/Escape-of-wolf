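; Wolf enemy Blueprint that patrols around its spawn point, chases a seen TopDownCharacter and bites it.
; Patrol loops AIMoveTo toward ground points found by randomized downward line traces within RadioDeMovimiento.
; PawnSensing starts the chase and plays the bite montage on arrival, while a retriggerable delay resumes patrol.
; Tick calls Daño, which traces between two sockets (passed as None) and applies damage while RealizandoAtaque is true.
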(event OnSeePawn(PawnSensing)
  (params (Pawn :type Pawn%20Object%20Reference))
  ;[1 1 1] persecucion
  (bind _astop_down_character (Utilities|Casting|CastToTopDownCharacter Pawn))
  (if (Class|AnimInstance|IsAnyMontagePlaying (Components|SkeletalMesh|GetAnimInstance (Variables|Character|GetMesh)))
    (Utilities|FlowControl|RetriggerableDelay 1.0 :!label _label)
    (CallFunction|Patrullar)
    (else
      (AI|AIMoveTo self "0, 0, 0" _astop_down_character 1e+01 false
        (:then
          (goto _label))
        (:OnSuccess
          (if (not (Class|AnimInstance|IsAnyMontagePlaying (Components|SkeletalMesh|GetAnimInstance (Variables|Character|GetMesh))))
            (Animation|Montage|PlayMontage (Variables|Character|GetMesh) "/Game/animacion/Wolf_RM_Attack_Bite_Front_Montage.Wolf_RM_Attack_Bite_Front_Montage")))))))

(event Custom|patrullar
  (bind _radio_de_movimiento (Variables|Default|Getradio%20de%20movimiento))
  (bind _radio_de_movimiento_2 (Variables|Default|Getradio%20de%20movimiento))
  (bind _radio_de_movimiento_3 (Variables|Default|Getradio%20de%20movimiento))
  (bind _radio_de_movimiento_4 (Variables|Default|Getradio%20de%20movimiento))
  (bind _ubicacion_inicial (Variables|Default|Getubicacion%20inicial))
  (bind _returnvalue (* _radio_de_movimiento_2 -1.0))
  (bind _returnvalue_2 (* _radio_de_movimiento_4 -1.0))
  (bind _returnvalue_3 (Math|Random|RandomFloatinRange _returnvalue _radio_de_movimiento))
  (bind _returnvalue_4 (Math|Random|RandomFloatinRange _returnvalue_2 _radio_de_movimiento_3))
  (bind _returnvalue_5 (+ _returnvalue_3 (.y _ubicacion_inicial)))
  (bind _returnvalue_6 (+ _returnvalue_4 (.x _ubicacion_inicial)))
  ;[1 1 1] patrullar
  (bind _outhit (Collision|LineTraceByChannel (Math|Vector|MakeVector _returnvalue_6 _returnvalue_5 5e+02) (Math|Vector|MakeVector _returnvalue_6 _returnvalue_5 -1e+02) "TraceTypeQuery1" false 0 "None" :!label _label))
  (AI|AIMoveTo self (.ImpactPoint (Collision|BreakHitResult _outhit)) 0 5.0 false
    (:OnSuccess
      (Utilities|FlowControl|Delay 2.0)
      (Development|PrintString "Gow")
      (goto _label))
    (:OnFail
      (CallFunction|Patrullar))))

(event EventBeginPlay
  (Variables|Default|Setubicacion%20inicial (Transformation|GetActorLocation self))
  ;[1 1 1] patrullar
  (bind _outhit (Collision|LineTraceByChannel (Math|Vector|MakeVector (+ (Math|Random|RandomFloatinRange (* (Variables|Default|Getradio%20de%20movimiento) -1.0) (Variables|Default|Getradio%20de%20movimiento)) (.x (Variables|Default|Getubicacion%20inicial))) (+ (Math|Random|RandomFloatinRange (* (Variables|Default|Getradio%20de%20movimiento) -1.0) (Variables|Default|Getradio%20de%20movimiento)) (.y (Variables|Default|Getubicacion%20inicial))) 5e+02) (Math|Vector|MakeVector (+ (Math|Random|RandomFloatinRange (* (Variables|Default|Getradio%20de%20movimiento) -1.0) (Variables|Default|Getradio%20de%20movimiento)) (.x (Variables|Default|Getubicacion%20inicial))) (+ (Math|Random|RandomFloatinRange (* (Variables|Default|Getradio%20de%20movimiento) -1.0) (Variables|Default|Getradio%20de%20movimiento)) (.y (Variables|Default|Getubicacion%20inicial))) -1e+02) "TraceTypeQuery1" false 0 "None" :!label _label))
  (AI|AIMoveTo self (.ImpactPoint (Collision|BreakHitResult _outhit)) 0 5.0 false
    (:OnSuccess
      (Utilities|FlowControl|Delay 2.0)
      (Development|PrintString "Gow")
      (goto _label))
    (:OnFail
      (CallFunction|Patrullar))))

(event EventTick
  (params (DeltaSeconds :type Float%20%28single-precision%29))
  (CallFunction|Daño "None" "None"))

(fn ConstructionScript)

(fn Daño
  (params (attack%20ini :type Name) (attack%20fin :type Name))
  (bind _mesh (Variables|Character|GetMesh))
  (if (Variables|Default|GetRealizando%20ataque)
    (bind (_outhit _returnvalue) (Collision|LineTraceByChannel (Transformation|GetSocketLocation _mesh attack%20ini) (Transformation|GetSocketLocation _mesh attack%20fin) "TraceTypeQuery1" false 0 "ForDuration"))
    (if _returnvalue
      (bind _astop_down_character (Utilities|Casting|CastToTopDownCharacter (.HitActor (Collision|BreakHitResult _outhit))))
      (Game|Damage|ApplyDamage _astop_down_character 8.0 (Game|GetInstigatorController _astop_down_character) self))))