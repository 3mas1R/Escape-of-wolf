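; BP_Iteam_attack is a spinning wolf-skull pickup that adds points to the Thief's Puntuacion score.
; An overlap on the skull component casts to Thief, adds the points, and destroys the actor only if Spawned is true.
; Tick rotates the actor every frame and feeds a Delay that destroys it about 30 seconds after ticking starts, regardless of Spawned.
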(event OnComponentBeginOverlap(animalSkulls_25_wolf)
  (params (OverlappedComponent :type Primitive%20Component%20Object%20Reference) (OtherActor :type Actor%20Object%20Reference) (OtherComp :type Primitive%20Component%20Object%20Reference) (OtherBodyIndex :type Integer) (bFromSweep :type Boolean) (SweepResult :type Hit%20Result%20Structure%20%28by%20ref%29))
  (bind _asthief (Utilities|Casting|CastToThief OtherActor))
  (Variables|/Game/TopDownBP/Blueprints/Thief.Thief_C|SetPuntuacion _asthief (+ (Variables|/Game/TopDownBP/Blueprints/Thief.Thief_C|GetPuntuacion _asthief) 100))
  (if (Variables|Default|Getspawned)
    (Actor|DestroyActor)))

(event EventBeginPlay)

(event Collision|EventActorBeginOverlap
  (params (OtherActor :type Actor%20Object%20Reference)))

(event EventTick
  (params (DeltaSeconds :type Float%20%28single-precision%29))
  (Transformation|AddActorLocalRotation "0,2.500000, 0" false false)
  (Utilities|FlowControl|Delay 3e+01)
  (Actor|DestroyActor))

(fn ConstructionScript)