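; BP_Iteam_Speed is a spinning pickup that gives the Thief a temporary walk-speed boost.
; Overlapping its mesh sets Bottomview, shows a Speed widget and raises MaxWalkSpeed, then after about five seconds resets speed and flag and destroys the actor.
; End overlap hides the pickup while the boost runs.
; Tick rotates it and re-triggers a delayed destroy every frame, so that timeout never completes while ticking.
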(event OnComponentEndOverlap(Pl_PowerUp_02)
  (params (OverlappedComponent :type Primitive%20Component%20Object%20Reference) (OtherActor :type Actor%20Object%20Reference) (OtherComp :type Primitive%20Component%20Object%20Reference) (OtherBodyIndex :type Integer))
  (Utilities|Casting|CastToThief OtherActor)
  (Rendering|SetActorHiddenInGame true)
  (Utilities|FlowControl|Delay 5.0))

(event OnComponentBeginOverlap(Pl_PowerUp_02)
  (params (OverlappedComponent :type Primitive%20Component%20Object%20Reference) (OtherActor :type Actor%20Object%20Reference) (OtherComp :type Primitive%20Component%20Object%20Reference) (OtherBodyIndex :type Integer) (bFromSweep :type Boolean) (SweepResult :type Hit%20Result%20Structure%20%28by%20ref%29))
  (bind _asthief (Utilities|Casting|CastToThief OtherActor))
  (Variables|/Game/TopDownBP/Blueprints/Thief.Thief_C|Setbottomview _asthief true)
  (bind _returnvalue (UserInterface|CreateWidget "/Game/ui/speed.speed_C"))
  (UserInterface|Viewport|AddtoViewport _returnvalue 0)
  (Variables|/Script/Engine.CharacterMovementComponent|SetMaxWalkSpeed (Variables|/Script/Engine.Character|GetCharacterMovement _asthief) 8e+02)
  (Utilities|FlowControl|Delay 5.1)
  (Variables|/Script/Engine.CharacterMovementComponent|SetMaxWalkSpeed (Variables|/Script/Engine.Character|GetCharacterMovement _asthief) 6e+02)
  (Variables|/Game/TopDownBP/Blueprints/Thief.Thief_C|Setbottomview _asthief false)
  (Actor|DestroyActor))

(event EventBeginPlay)

(event Collision|EventActorBeginOverlap
  (params (OtherActor :type Actor%20Object%20Reference)))

(event EventTick
  (params (DeltaSeconds :type Float%20%28single-precision%29))
  (Transformation|AddActorLocalRotation "0,2.500000, 0" false false)
  (Utilities|FlowControl|RetriggerableDelay 1e+01)
  (Actor|DestroyActor))

(fn ConstructionScript)